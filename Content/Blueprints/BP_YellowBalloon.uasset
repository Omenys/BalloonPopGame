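; BP_YellowBalloon is a clickable balloon actor that rises, swells with clicks and then disappears.
; It starts at a reduced scale and moves up by MoveSpeed every Tick, without delta-time scaling or sweep.
; BalloonClicks enlarges it and decrements Clicks while any remain, then destroys the actor on the following call.
; Nothing in this Blueprint calls BalloonClicks itself.
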(event `self.ReceiveBeginPlay`
  (`self.SetActorScale3D` (0.2 0.2 0.2)))

(event `self.ReceiveTick`
  (params (DeltaSeconds :type "Float (single-precision)"))
  (`self.K2_SetActorLocation` (+ (`KismetMathLibrary.MakeVector` (.x (`self.K2_GetActorLocation`)) (.y (`self.K2_GetActorLocation`)) (.z (`self.K2_GetActorLocation`))) (`KismetMathLibrary.MakeVector` 0.0 0.0 (`self.moveSpeed`)))))

(fn `BalloonClicks`
  (if (> (`self.clicks`) 0)
    (`self.SetActorScale3D` (+ (`SceneComponent.K2_GetComponentScale` (`self.Yellow_Balloon`)) (0.02 0.02 0.02)))
    (set `self.clicks` (- (`self.clicks`) 1))
    (else
      (`self.K2_DestroyActor`))))

(fn `UserConstructionScript`)