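; BP_ClickInput handles mouse clicks on balloons and shows the cursor when play begins.
; Each left click runs two complex visibility traces under the cursor, casting the hit actor to red and then yellow balloon types.
; A red hit destroys the balloon and adds RedPoints to Score.
; A yellow hit only calls BalloonClicks on that balloon, with no score change here.
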(event `self.ReceiveBeginPlay`
  (set `self.bShowMouseCursor` true))

(event `Key|LeftMouseButton`
  (params (Key :type "Key Structure"))
  (bind (_bblockinghit _binitialoverlap _time _distance _location _impactpoint _normal _impactnormal _physmat _hitactor) (`GameplayStatics.BreakHitResult` (`self.GetHitResultUnderCursorByChannel` "TraceTypeQuery1")))
  (:`Pressed`
    (`|ExecutionSequence`
      (:`then_0`
        (bind _asbp_red_balloon (cast `/Game/Blueprints/BP_RedBalloon` _hitactor))
        (`KismetSystemLibrary.PrintString` "")
        (`/Game/Blueprints/BP_RedBalloon.DestroyRedBalloon` _asbp_red_balloon)
        (set `self.score` (+ (`self.score`) (`self.redPoints`))))
      (:`then_1`
        (bind _asbp_yellow_balloon (cast `/Game/Blueprints/BP_YellowBalloon` _hitactor))
        (`/Game/Blueprints/BP_YellowBalloon.BalloonClicks` _asbp_yellow_balloon)))))

(fn `UserConstructionScript`)